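; BP_Flasks is a generator actor that produces a randomized arrangement of flask props for the chemistry room set.
; The Construction Script loops over six flask mesh components and sets each one's visibility from a weighted random bool driven by the RandomVis chance.
; The event graph holds only disabled placeholder events, so the actor has no runtime logic.
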(event EventBeginPlay)

(event Collision|EventActorBeginOverlap
  (params (OtherActor :type Actor%20Object%20Reference)))

(event EventTick
  (params (DeltaSeconds :type Float%20%28single-precision%29)))

(fn ConstructionScript
  (for _array_element (Utilities|Array|MakeArray (Variables|Default|GetSM_Flask_5) (Variables|Default|GetSM_Flask_6) (Variables|Default|GetSM_Flask_7) (Variables|Default|GetSM_Flask_2) (Variables|Default|GetSM_Flask_3) (Variables|Default|GetSM_Flask_4))
    (Rendering|SetVisibility _array_element (Math|Random|RandomBoolwithWeight (Variables|Default|GetRandom%20Vis)) false)))